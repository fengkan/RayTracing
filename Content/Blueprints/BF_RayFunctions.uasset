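; BF_RayFunctions is a set of helper functions for a ray struct defined by Start and End points.
; RayOrigin returns Start, and RayDirection returns the unnormalized vector End minus Start.
; RayPointAtParameter combines both as origin plus direction times T, so T runs from 0 at Start to 1 at End, with no clamping.
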(fn RayDirection
  (params (ray :type S%20Ray%20Structure))
  (bind (_start _end) (Utilities|Struct|BreakS_Ray ray))
  (return (- _end _start)))

(fn RayPointatParameter
  (params (t :type Float%20%28single-precision%29) (ray :type S%20Ray%20Structure))
  (return (+ (CallFunction|RayOrigin ray) (* (CallFunction|RayDirection ray) t))))

(fn RayOrigin
  (params (ray :type S%20Ray%20Structure))
  (return (.start (Utilities|Struct|BreakS_Ray ray))))