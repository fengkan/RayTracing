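; BP_HitableList is a hitable made up of a list of hitables, used for ray intersection in a ray-tracing setup.
; Hit tests the ray R against every List entry, shrinking the upper bound to the closest hit so far.
; It returns whether anything was hit plus the nearest hit record.
; Child tests use a hardcoded minimum distance, so the TMin input is ignored.
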(fn ConstructionScript
  (|CallParentFunction))

(fn Hit
  (params (t_min :type Float%20%28single-precision%29) (t_max :type Float%20%28single-precision%29) (r :type S%20Ray%20Structure))
  (LocalVariables|SetHitAnything false)
  (LocalVariables|SetClosestSoFar t_max)
  (bind _index (Utilities|FlowControl|ForLoopwithBreak 0 (- (Utilities|Array|Length (Variables|Default|Getlist)) 1))
    (:LoopBody
      (bind (_result _rec) (Default|Hit (Utilities|Array|Get(acopy) (Variables|Default|Getlist) _index) 0.001 (LocalVariables|GetClosestSoFar) r))
      (if _result
        (LocalVariables|SetHitAnything true)
        (LocalVariables|SetClosestSoFar (.t (Utilities|Struct|BreakS_HitRecord _rec)))
        (LocalVariables|SettempRec _rec)))
    (:Completed
      (return (LocalVariables|GetHitAnything) (LocalVariables|GettempRec)))))