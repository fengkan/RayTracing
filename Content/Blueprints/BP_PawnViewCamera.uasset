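; BP_PawnViewCamera is a free-fly camera pawn that keeps the mouse cursor visible and click events enabled.
; Turn and LookUp axes adjust actor yaw and pitch only while the right mouse button is held.
; MoveForward and MoveRight store scaled axis values, which Tick rotates by the root's pitch and yaw to offset the location.
; Movement follows the view direction without sweep, and its step is per frame, unscaled by delta time.
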(event EventBeginPlay
  (bind _returnvalue (Game|GetPlayerController 0))
  (Variables|/Script/Engine.PlayerController|SetbShowMouseCursor _returnvalue true)
  (Variables|/Script/Engine.PlayerController|SetbEnableClickEvents _returnvalue true))

(event EventTick
  (params (DeltaSeconds :type Float%20%28single-precision%29))
  (bind _defaultsceneroot (Variables|Default|GetDefaultSceneRoot))
  (bind _returnvalue (Transformation|GetWorldRotation _defaultsceneroot))
  (bind (_roll _pitch _yaw) (Math|Rotator|BreakRotator _returnvalue))
  (Transformation|SetActorLocation (+ (* (Math|Vector|RotateVector (Math|Vector|MakeVector (Variables|Default|GetForwardAxis) (Variables|Default|GetRightAxis) 0.0) (Math|Rotator|MakeRotator 0.0 _pitch _yaw)) 1e+02) (Transformation|GetWorldLocation _defaultsceneroot)) false false))

(event Input|AxisEvents|InputAxisMoveRight
  (params (AxisValue :type Float%20%28single-precision%29))
  (Variables|Default|SetRightAxis (/ AxisValue 4.0)))

(event Input|AxisEvents|InputAxisTurn
  (params (AxisValue :type Float%20%28single-precision%29))
  (bind _returnvalue (Transformation|GetActorRotation))
  (bind (_roll _pitch _yaw) (Math|Rotator|BreakRotator _returnvalue))
  (if (Game|Player|IsInputKeyDown (Game|GetPlayerController 0) "RightMouseButton")
    (Transformation|SetActorRotation (Math|Rotator|MakeRotator _roll _pitch (+ _yaw (* AxisValue 1.0))))))

(event Input|AxisEvents|InputAxisLookUp
  (params (AxisValue :type Float%20%28single-precision%29))
  (bind _returnvalue (Transformation|GetActorRotation))
  (bind (_roll _pitch _yaw) (Math|Rotator|BreakRotator _returnvalue))
  (if (Game|Player|IsInputKeyDown (Game|GetPlayerController 0) "RightMouseButton")
    (Transformation|SetActorRotation (Math|Rotator|MakeRotator _roll (+ _pitch (* AxisValue -1.0)) _yaw))))

(event Input|AxisEvents|InputAxisMoveForward
  (params (AxisValue :type Float%20%28single-precision%29))
  (Variables|Default|SetForwardAxis (/ AxisValue 4.0)))

(fn ConstructionScript)