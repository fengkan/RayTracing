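; BP_Board is a clickable grid board, standing in the Y-Z plane and sized by its Row and Column counts.
; The construction script scales the static mesh to those counts.
; On a mesh click, it takes the mouse position from BP_RTController, converts it to cell indices using fixed-size cells centered on the actor, with the vertical index flipped, and passes them to CallClicked.
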(event OnClicked(StaticMesh)
  (params (TouchedComponent :type Primitive%20Component%20Object%20Reference) (ButtonPressed :type Key%20Structure))
  (bind _returnvalue (Transformation|GetActorLocation))
  (bind _asbp_rtcontroller (Utilities|Casting|CastToBP_RTController (Game|GetPlayerController 0)))
  (bind _hit_result_impact_point (Default|GetMouseClickedPosition _asbp_rtcontroller))
  (Default|CallClicked (.ReturnValue (Math|Float|Division(WholeandRemainder) (- (.y _hit_result_impact_point) (- (.y _returnvalue) (* (/ (Math|Conversions|ToFloat(Integer) (Variables|Default|Getcolumn)) 2.0) 1e+01))) 1e+01)) (- (- (Variables|Default|Getrow) 1) (.ReturnValue (Math|Float|Division(WholeandRemainder) (- (.z _hit_result_impact_point) (- (.z _returnvalue) (* (/ (Math|Conversions|ToFloat(Integer) (Variables|Default|Getrow)) 2.0) 1e+01))) 1e+01)))))

(fn ConstructionScript
  (Transformation|SetWorldScale3D (Variables|Default|GetStaticMesh) (Math|Vector|MakeVector 0.1 (* (Variables|Default|Getcolumn) 0.1) (* (Variables|Default|Getrow) 0.1))))