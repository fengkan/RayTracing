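; A sphere actor that a ray can be tested against, as a hitable object for ray tracing written in Blueprint.
; The construction script scales the static mesh from Radius, so the visible sphere is meant to match the analytic one.
; Hit solves the ray-sphere quadratic around the actor location, trying the nearer root before the farther within TMin and TMax.
; A hit returns a record with distance parameter, point and radius-normalized normal.
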(fn ConstructionScript
  (bind _radius (Variables|Default|Getradius))
  (bind _returnvalue (/ _radius 1e+02))
  (bind _returnvalue_2 (* _returnvalue 2.0))
  (Transformation|SetWorldScale3D (Variables|Default|GetStaticMesh) (Math|Vector|MakeVector _returnvalue_2 _returnvalue_2 _returnvalue_2)))

(fn Hit
  (params (t_min :type Float%20%28single-precision%29) (t_max :type Float%20%28single-precision%29) (r :type S%20Ray%20Structure))
  (bind _direction (CallFunction|RayDirection r))
  (bind _radius (Variables|Default|Getradius))
  (LocalVariables|SetlocalR r)
  (LocalVariables|SetlocalTMin t_min)
  (LocalVariables|SetlocalTMax t_max)
  (Utilities|FlowControl|Sequence
    (:then_0
      (LocalVariables|Setoc (- (CallFunction|RayOrigin r) (Transformation|GetActorLocation)))
      (LocalVariables|Seta (Math|Vector|DotProduct _direction _direction))
      (LocalVariables|Setb (Math|Vector|DotProduct _direction (LocalVariables|Getoc)))
      (LocalVariables|Setc (- (Math|Vector|DotProduct (LocalVariables|Getoc) (LocalVariables|Getoc)) (* _radius _radius)))
      (LocalVariables|Setdiscriminant (- (* (LocalVariables|Getb) (LocalVariables|Getb)) (* (LocalVariables|Geta) (LocalVariables|Getc)))))
    (:then_1
      (if (> (LocalVariables|Getdiscriminant) 0.0)
        (LocalVariables|Settemp (/ (- (- 0.0 (LocalVariables|Getb)) (Math|Float|Sqrt (- (* (LocalVariables|Getb) (LocalVariables|Getb)) (* (LocalVariables|Geta) (LocalVariables|Getc))))) (LocalVariables|Geta)))
        (if (and (< (LocalVariables|Gettemp) (LocalVariables|GetlocalTMax)) (> (LocalVariables|Gettemp) (LocalVariables|GetlocalTMin)))
          (return true (Utilities|Struct|MakeS_HitRecord (LocalVariables|Gettemp) (CallFunction|RayPointatParameter (LocalVariables|Gettemp) (LocalVariables|GetlocalR)) (/ (- (CallFunction|RayPointatParameter (LocalVariables|Gettemp) (LocalVariables|GetlocalR)) (Transformation|GetActorLocation)) (Variables|Default|Getradius))))
          (else
            (LocalVariables|Settemp (/ (+ (- 0.0 (LocalVariables|Getb)) (Math|Float|Sqrt (- (* (LocalVariables|Getb) (LocalVariables|Getb)) (* (LocalVariables|Geta) (LocalVariables|Getc))))) (LocalVariables|Geta)))
            (if (and (< (LocalVariables|Gettemp) (LocalVariables|GetlocalTMax)) (> (LocalVariables|Gettemp) (LocalVariables|GetlocalTMin)))
              (return true (Utilities|Struct|MakeS_HitRecord (LocalVariables|Gettemp) (CallFunction|RayPointatParameter (LocalVariables|Gettemp) (LocalVariables|GetlocalR)) (/ (- (CallFunction|RayPointatParameter (LocalVariables|Gettemp) (LocalVariables|GetlocalR)) (Transformation|GetActorLocation)) (Variables|Default|Getradius))))
              (else
                (return false "")))))
        (else
          (return false ""))))))